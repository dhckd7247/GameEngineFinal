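; EnemyBP is an enemy that damages the hero for as long as the two overlap.
; On BeginPlay it sets its HP and caches the ShooterGameMode.
; Overlap with a HeroBP deals damage immediately, then repeats it on a looping timer by function name until the overlap ends.
; No logic here changes the enemy's own HP or uses the cached game mode afterward.
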(event Custom|DecreaseHeroHP
  (Default|DecreaseHP (stale Collision|EventActorBeginOverlap _ashero_bp) 2e+01))

(event Collision|EventActorBeginOverlap
  (params (OtherActor :type Actor%20Object%20Reference))
  (bind _ashero_bp (Utilities|Casting|CastToHeroBP OtherActor))
  (CallFunction|DecreaseHeroHP)
  (Utilities|Time|SetTimerbyFunctionName 0 "DecreaseHeroHP" 0.2 true))

(event Collision|EventActorEndOverlap
  (params (OtherActor :type Actor%20Object%20Reference))
  (Utilities|Casting|CastToHeroBP OtherActor)
  (Utilities|Time|ClearTimerbyFunctionName 0 "DecreaseHeroHP"))

(event EventBeginPlay
  (Variables|Default|SetHP 1e+02)
  (bind _asshooter_game_mode (Utilities|Casting|CastToShooterGameMode (Game|GetGameMode)))
  (Variables|Default|SetGameMode _asshooter_game_mode))

(fn ConstructionScript)